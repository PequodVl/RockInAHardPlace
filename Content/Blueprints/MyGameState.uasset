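; MyGameState is the game state Blueprint, providing a helper that spawns an item into the world in front of a given actor.
; SpawnItemFromActor places the spawn point slightly above and ahead of the actor, matching its rotation, and optionally snaps it down with a short Visibility line trace.
; It spawns the class reported by the item object, passes that object to the new actor and enables physics simulation.
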(event EventBeginPlay)

(event EventTick
  (params (DeltaSeconds :type Float%20%28single-precision%29)))

(fn ConstructionScript)

(fn SpawnItemfromActor
  (params (ItemObject :type Bp%20Item%20Object%20Object%20Reference) (Actor :type Actor%20Object%20Reference) (GroundClamp :type Boolean))
  (bind _itemclass (Default|GetItemClass ItemObject))
  (Utilities|FlowControl|Sequence
    (:then_0
      (LocalVariables|SetSpawnRotation%20%28local%29 (Transformation|GetActorRotation Actor))
      (bind _output_get (LocalVariables|SetSpawnLocation%20%28local%29 (+ (+ (Transformation|GetActorLocation Actor) "0.000000,0.000000,50.000000") (* (Transformation|GetActorForwardVector Actor) 100))))
      (if GroundClamp
        (bind (_outhit _returnvalue) (Collision|LineTraceByChannel _output_get (- (LocalVariables|GetSpawnLocation%20%28local%29) "0.000000,0.000000,100.000000") "TraceTypeQuery1" false 0 "None"))
        (if _returnvalue
          (LocalVariables|SetSpawnLocation%20%28local%29 (.Location (Collision|BreakHitResult _outhit))))))
    (:then_1
      (bind _returnvalue_2 (Game|SpawnActorfromClass :Class _itemclass :SpawnTransform (Math|Transform|MakeTransform (LocalVariables|GetSpawnLocation%20%28local%29) (LocalVariables|GetSpawnRotation%20%28local%29) "1.000000,1.000000,1.000000") :CollisionHandlingOverride "Undefined" :TransformScaleMethod "MultiplyWithRoot" :ItemClass _itemclass :ItemName "MissingItemNameErr" :ItemImage "/Game/Blueprints/items/Weapons/Scar_beta/Scar_beta.Scar_beta" :ItemObject ItemObject :Instigator 0))
      (Default|SetSimulatePhysics _returnvalue_2))))