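; Damage-test mannequin actor that shows incoming damage on in-world text displays.
; On AnyDamage it plays a 2D hit sound, writes the remaining health and the damage amount to two text renders, then subtracts the damage.
; When health drops below zero, it resets to full and refreshes the health display.
; The SendDamage event is present but empty.
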(event Custom|SendDamage_1
  (params (Amount :type Float%20%28double-precision%29) (Type :type Name :default "None")))

(event EventBeginPlay)

(event Collision|EventActorBeginOverlap
  (params (OtherActor :type Actor%20Object%20Reference)))

(event EventTick
  (params (DeltaSeconds :type Float%20%28single-precision%29)))

(event Game|Damage|EventAnyDamage
  (params (Damage :type Float%20%28single-precision%29) (DamageType :type Damage%20Type%20Object%20Reference) (InstigatedBy :type Controller%20Object%20Reference) (DamageCauser :type Actor%20Object%20Reference))
  (Audio|PlaySound2D "/Game/untitled_category/Sound/HitSound.HitSound" 1.0 1.0 0.0 0 0)
  (Rendering|Components|TextRender|SetText (Variables|Default|GetTextRender) (Utilities|Text|ToText(Float) (- (Variables|Default|GetHealth) Damage) "HalfToEven"))
  (Rendering|Components|TextRender|SetText (Variables|Default|GetTextRender1) (Utilities|Text|ToText(Float) Damage "HalfToEven"))
  (Variables|Default|SetHealth (- (Variables|Default|GetHealth) Damage))
  (if (< (Variables|Default|GetHealth) 0.0)
    (bind _output_get (Variables|Default|SetHealth 1e+03))
    (Rendering|Components|TextRender|SetText (Variables|Default|GetTextRender) (Utilities|Text|ToText(Float) _output_get "HalfToEven"))))

(fn ConstructionScript)