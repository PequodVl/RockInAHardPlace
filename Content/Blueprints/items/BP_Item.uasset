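; Base pickup item actor that shows a screen-space name and icon widget while under the player's cursor.
; Interaction adds its ItemObject to the player's inventory, destroying the actor on success.
; Without a valid ItemObject on BeginPlay, it takes one from the empty GetDefaultItemObject stub and enables physics on its skeletal or static mesh.
; Hits play a drop sound scaled by Sphere velocity, throttled by a delayed DoOnce reset.
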(event Custom|SetSimulatePhysics
  (bind _skeletalmesh (Variables|Default|GetSkeletalMesh))
  (bind _staticmesh (Variables|Default|GetStaticMesh))
  (if (Variables|Default|GetUsesSkeletalMesh)
    (Collision|SetCollisionProfileName _skeletalmesh "DroppedItem" true :!class /Script/Engine.PrimitiveComponent)
    (Physics|SetSimulatePhysics _skeletalmesh true)
    (Variables|Default|SetDefaultSceneRoot _skeletalmesh)
    (else
      (Collision|SetCollisionProfileName _staticmesh "DroppedItem" true :!class /Script/Engine.PrimitiveComponent)
      (Physics|SetSimulatePhysics _staticmesh true)
      (Variables|Default|SetDefaultSceneRoot _staticmesh))))

(event Custom|SetNotSimulatePhysics
  (if (Variables|Default|GetUsesSkeletalMesh)
    (Physics|SetSimulatePhysics (Variables|Default|GetSkeletalMesh) false)
    (else
      (Physics|SetSimulatePhysics (Variables|Default|GetStaticMesh) false))))

(event EventBeginPlay
  (if (not (Utilities|IsValid (Variables|ItemInfo|GetItemObject)))
    (bind _itemobject (CallFunction|GetDefaultItemObject))
    (Variables|ItemInfo|SetItemObject _itemobject)
    (CallFunction|SetSimulatePhysics)))

(event EventOnItemIsinCursor
  (params (Player :type BP%20True%20Fps%20Character%20Object%20Reference))
  (bind _itemobject (Variables|ItemInfo|GetItemObject))
  (Variables|Default|GetTheInteractionWidgetComponent
    (:then)
    (:else
      (bind _returnvalue (UserInterface|CreateWidget "/Game/Blueprints/Interface/IW_Weapon.IW_Weapon_C" (.AsPlayer%20Controller (Utilities|Casting|CastToPlayerController (Pawn|GetController Player))) (Variables|/Game/Blueprints/items/Bp_Item_Object.Bp_Item_Object_C|GetItemName _itemobject) (Variables|/Game/Blueprints/items/Bp_Item_Object.Bp_Item_Object_C|GetIcon _itemobject)))
      (bind _returnvalue_2 (AddComponent|AddWidgetComponent false))
      (bind _output_get (Variables|Default|SetTheInteractionWidgetComponent _returnvalue_2))
      (UserInterface|SetWidget _output_get _returnvalue)
      (Class|WidgetComponent|SetWidgetSpace _output_get "Screen")
      (Class|WidgetComponent|SetDrawatDesiredSize _output_get true)
      (Collision|SetCollisionEnabled _output_get "NoCollision")
      (Transformation|AttachComponentToComponent _output_get (CallFunction|GetInteractionTextAttach) "None" "SnapToTarget" "SnapToTarget" "SnapToTarget" true))))

(event EventOnItemlostCursor
  (bind _theinteractionwidgetcomponent (Variables|Default|GetTheInteractionWidgetComponent)
    (:then
      (Components|DestroyComponent _theinteractionwidgetcomponent))
    (:else)))

(event EventOnInteracted
  (params (Player :type BP%20True%20Fps%20Character%20Object%20Reference))
  (bind _inventorycomponent (Variables|/Game/Blueprints/Character/BP_TrueFpsCharacter.BP_TrueFpsCharacter_C|GetInventoryComponent Player))
  (bind _added (Default|TryAddItem _inventorycomponent (Variables|ItemInfo|GetItemObject) (Variables|/Game/Blueprints/items/Inventory/InventoryComponent.InventoryComponent_C|GetItemsInInventory _inventorycomponent)))
  (if _added
    (Actor|DestroyActor)
    (Default|PickUpSuccessful Player)))

(event Collision|EventHit
  (params (MyComp :type Primitive%20Component%20Object%20Reference) (Other :type Actor%20Object%20Reference) (OtherComp :type Primitive%20Component%20Object%20Reference) (bSelfMoved :type Boolean) (HitLocation :type Vector :default "0, 0, 0") (HitNormal :type Vector :default "0, 0, 0") (NormalImpulse :type Vector :default "0, 0, 0") (Hit :type Hit%20Result%20Structure%20%28by%20ref%29))
  (Utilities|FlowControl|DoOnce false :!label _label
    (:Completed
      (bind _returnvalue (Physics|GetPhysicsLinearVelocity (Variables|Default|GetSphere) "None"))
      (Utilities|FlowControl|Sequence
        (:then_0
          (Audio|PlaySoundatLocation (Variables|Default|GetDropSound) HitLocation "0, 0, 0" (Math|Float|Clamp(Float) (/ (Math|Vector|VectorLength _returnvalue) 1.2e+03)) 1.0 0.0 0 0 0 0))
        (:then_1
          (Utilities|FlowControl|Delay 0.4)
          (goto _label Reset))))))

(fn ConstructionScript)

(fn GetInteractionText
  (return ""))

(fn GetInteractionTextAttach
  (return (Variables|Default|GetSphere)))

(fn GetDefaultItemObject
  (return 0))