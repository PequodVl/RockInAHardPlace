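; BP__ScarBeta is a SCAR gun item that supplies the default data object for this weapon.
; GetDefaultItemObject constructs a Bp_Weapon_Object with a hard-coded fire rate and weapon length, filling ammo, handle transform, dimensions, icon, class and name from the actor's variables.
; The construction script only calls the parent, and the event graph holds only disabled placeholder events.
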(event Collision|EventActorBeginOverlap
  (params (OtherActor :type Actor%20Object%20Reference)))

(event EventTick
  (params (DeltaSeconds :type Float%20%28single-precision%29)))

(fn ConstructionScript
  (|CallParentFunction))

(fn GetDefaultItemObject
  (bind _returnvalue (Game|ConstructObjectfromClass self "/Game/Blueprints/items/Guns/Bp_Weapon_Object.Bp_Weapon_Object_C" 0 5.5e+02 6 (Variables|Default|GetCurrentAmmo) (Variables|Default|GetMaxAmmo) (Variables|Default|GetWeaponhandleRotation) (Variables|Default|GetWeaponHandleOffset) (Variables|Default|GetDimensions) (Variables|Default|GetItemImage) (Variables|Default|GetItemClass) (Variables|Default|GetItemName)))
  (return _returnvalue))