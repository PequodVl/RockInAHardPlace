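; Gun item Blueprint that fires projectiles and handles physical magazine actors.
; FireEvent runs a gated, retriggerable-delay loop paced by Firerate until StopFireEvent, spending weapon-object ammo on muzzle-socket projectiles, sound, effects and animation.
; Magazines spawn on the gun or player's hand, with separate reload events to re-parent and swap them.
; Reload only drops the current magazine, saving its ammo and enabling physics.
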(event Custom|FireEvent
  (params (Player :type BP%20True%20Fps%20Character%20Object%20Reference))
  (bind _itemobject (Variables|Default|GetItemObject))
  (bind _skeletalmesh (Variables|Default|GetSkeletalMesh))
  (bind _returnvalue (Transformation|GetSocketTransform _skeletalmesh "MuzzleSocket" "RTS_World"))
  (bind _asbp_weapon_object (Utilities|Casting|CastToBp_Weapon_Object _itemobject))
  (bind _currentammo (Variables|/Game/Blueprints/items/Weapons/Bp_Weapon_Object.Bp_Weapon_Object_C|GetCurrentAmmo _asbp_weapon_object))
  (bind _firerate (Variables|/Game/Blueprints/items/Weapons/Bp_Weapon_Object.Bp_Weapon_Object_C|GetFirerate _asbp_weapon_object))
  (bind _returnvalue_2 (> _currentammo 0))
  (bind _returnvalue_3 (/ 6e+01 _firerate))
  (if (<= (Variables|Default|GetDelayToFire) 0.0)
    (if _returnvalue_2
      (Utilities|FlowControl|Sequence
        (:then_0
          (goto _label Open))
        (:then_1
          (Utilities|FlowControl|Gate true :!label _label
            (:Exit
              (Utilities|FlowControl|Sequence
                (:then_0
                  (Variables|Default|SetDelayToFire _returnvalue_3)
                  (if _returnvalue_2
                    (Utilities|FlowControl|Sequence
                      (:then_0
                        (Math|Integer|DecrementInt _currentammo
                          (:%20%20
                            (if true
                              (Audio|Components|Audio|Play (Variables|Default|GetMuzzleAudio) 0.0)
                              (Game|SpawnActorfromClass "/Game/Blueprints/items/Weapons/BP_Projectile.BP_Projectile_C" (Math|Transform|MakeTransform (.location _returnvalue) (.rotation _returnvalue) "0.200000,0.200000,0.200000") "Undefined" "MultiplyWithRoot" 0 0)
                              (Effects|SpawnEmitterAttached "/Game/InfinityBladeEffects/Effects/FX_Combat_Base/Impact/P_Impact_Player_Fire_Strong.P_Impact_Player_Fire_Strong" _skeletalmesh "MuzzleSocket")
                              (Components|Animation|PlayAnimation (Variables|Default|GetSkeletalMesh) (.gunfire (Variables|Default|GetAnimVarStructure)) false)))))
                      (:then_1
                        (Default|WeaponHasFired Player)))))
                (:then_1
                  (Utilities|FlowControl|RetriggerableDelay _returnvalue_3)
                  (Variables|Default|SetDelayToFire 0.0)
                  (goto _label))))))))))

(event Custom|StopFireEvent
  (bind _itemobject (Variables|Default|GetItemObject))
  (bind _skeletalmesh (Variables|Default|GetSkeletalMesh))
  (bind _returnvalue (Transformation|GetSocketTransform _skeletalmesh "MuzzleSocket" "RTS_World"))
  (bind _asbp_weapon_object (Utilities|Casting|CastToBp_Weapon_Object _itemobject))
  (bind _currentammo (Variables|/Game/Blueprints/items/Weapons/Bp_Weapon_Object.Bp_Weapon_Object_C|GetCurrentAmmo _asbp_weapon_object))
  (bind _firerate (Variables|/Game/Blueprints/items/Weapons/Bp_Weapon_Object.Bp_Weapon_Object_C|GetFirerate _asbp_weapon_object))
  (bind _returnvalue_2 (/ 6e+01 _firerate))
  (Utilities|FlowControl|Gate true) ; enters at Close
)

(event Custom|DropMag
  (Variables|/Game/Blueprints/items/Magazines/Bp_Magazine_object.Bp_Magazine_object_C|SetCurrentAmmo (.AsBp%20Magazine%20Object (Utilities|Casting|CastToBp_Magazine_object (Variables|/Game/Blueprints/items/BP_Item.BP_Item_C|GetItemObject (Variables|Default|GetCurrentMag)))) (Variables|/Game/Blueprints/items/Weapons/Bp_Weapon_Object.Bp_Weapon_Object_C|GetCurrentAmmo (.AsBp%20Weapon%20Object (Utilities|Casting|CastToBp_Weapon_Object (Variables|Default|GetItemObject)))))
  (Transformation|DetachFromActor (Variables|Default|GetCurrentMag) "KeepWorld" "KeepWorld" "KeepWorld")
  (Collision|SetCollisionProfileName (Variables|/Game/Blueprints/items/BP_Item.BP_Item_C|GetStaticMesh (Variables|Default|GetCurrentMag)) "DroppedItem" true :!class /Script/Engine.PrimitiveComponent)
  (Physics|SetSimulatePhysics (Variables|/Game/Blueprints/items/BP_Item.BP_Item_C|GetStaticMesh (Variables|Default|GetCurrentMag)) true)
  (Variables|Default|SetCurrentMag 0))

(event Custom|Reload
  (CallFunction|DropMag))

(event Custom|CreateMagazine
  (params (IsForReload :type Boolean) (PlayerForReload :type BP%20True%20Fps%20Character%20Object%20Reference))
  (bind _mesh (Variables|/Script/Engine.Character|GetMesh PlayerForReload))
  (bind _itemobject (Variables|Default|GetItemObject))
  (bind _asbp_weapon_object (Utilities|Casting|CastToBp_Weapon_Object _itemobject))
  (bind _defaultmag (Variables|/Game/Blueprints/items/Weapons/Bp_Weapon_Object.Bp_Weapon_Object_C|GetDefaultMag _asbp_weapon_object))
  (if IsForReload
    (bind _returnvalue (Game|SpawnActorfromClass :Class _defaultmag :SpawnTransform (Transformation|GetSocketTransform (Variables|/Script/Engine.Character|GetMesh PlayerForReload) "GrabBone_L" "RTS_World") :CollisionHandlingOverride "Undefined" :TransformScaleMethod "MultiplyWithRoot" :Owner self :ItemClass _defaultmag :ItemName "Scar Magazine" :ItemImage "/Game/Blueprints/items/Weapons/Scar_beta/Scar_beta.Scar_beta" :ItemObject 0 :UsesSkeletalMesh true :Instigator 0))
    (Default|SetNotSimulatePhysics _returnvalue)
    (Transformation|AttachComponentToComponent _returnvalue _mesh "GrabBone_L" "SnapToTarget" "SnapToTarget" "KeepWorld" true)
    (Transformation|SetActorTransform _returnvalue (Transformation|GetSocketTransform _mesh "GrabBone_L" "RTS_World"))
    (Variables|Default|SetFutureMag _returnvalue)
    (else
      (bind _returnvalue_2 (Game|SpawnActorfromClass :Class _defaultmag :SpawnTransform (Transformation|GetSocketTransform (Variables|Default|GetSkeletalMesh) "MagazineSocket" "RTS_World") :CollisionHandlingOverride "Undefined" :TransformScaleMethod "MultiplyWithRoot" :Owner self :ItemClass _defaultmag :ItemName "Scar Magazine" :ItemImage "/Game/Blueprints/items/Weapons/Scar_beta/Scar_beta.Scar_beta" :ItemObject 0 :UsesSkeletalMesh true :Instigator 0))
      (Default|SetNotSimulatePhysics _returnvalue_2)
      (Transformation|AttachComponentToComponent _returnvalue_2 (Variables|Default|GetSkeletalMesh) "MagazineSocket" "SnapToTarget" "SnapToTarget" "KeepWorld" true)
      (Variables|Default|SetCurrentMag _returnvalue_2))))

(event Custom|AttachNewMag
  (bind _futuremag (Variables|Default|GetFutureMag))
  (Transformation|DetachFromActor _futuremag "KeepWorld" "KeepWorld" "KeepWorld")
  (Transformation|AttachComponentToComponent _futuremag (Variables|Default|GetSkeletalMesh) "MagazineSocket" "SnapToTarget" "SnapToTarget" "KeepWorld" true))

(event Custom|ParentOldMag
  (bind _currentmag (Variables|Default|GetCurrentMag))
  (Transformation|DetachFromActor _currentmag "KeepWorld" "KeepWorld" "KeepWorld")
  (Transformation|AttachComponentToComponent _currentmag (Variables|/Script/Engine.Character|GetMesh (stale Custom|CreateMagazine PlayerForReload)) "DEF-hand_L" "KeepWorld" "KeepWorld" "KeepWorld" true))

(event Custom|SetNewMagAsCurrent
  (Variables|Default|SetCurrentMag (Variables|Default|GetFutureMag)))

(event EventDestroyed
  (Actor|DestroyActor (Variables|Default|GetCurrentMag)))

(event EventBeginPlay
  (bind _shotsound (Variables|Default|GetShotSound))
  (|CallParentFunction)
  (Audio|Components|Audio|SetSound (Variables|Default|GetMuzzleAudio) (Utilities|Array|Get(acopy) _shotsound (Math|Random|RandomInteger (Utilities|Array|Length _shotsound))))
  (CallFunction|CreateMagazine false))

(fn ConstructionScript
  (|CallParentFunction))

(fn GetDefaultItemObject
  (bind _returnvalue (Game|ConstructObjectfromClass self "/Game/Blueprints/items/Weapons/Bp_Weapon_Object.Bp_Weapon_Object_C" "/Game/Blueprints/items/Weapons/Scar_beta/ScarBetaShotSound.ScarBetaShotSound" 1e+01 1 0 0 "0.000000,0.000000,0.000000" "0.000000,0.000000,0.000000" "/Game/Blueprints/items/Magazines/BP_Item_magazine.BP_Item_magazine_C" (Utilities|Array|MakeArray "NewEnumerator0") (Utilities|Struct|MakeIntPoint 1 1) 0 0 "GunNonExistant"))
  (return _returnvalue))