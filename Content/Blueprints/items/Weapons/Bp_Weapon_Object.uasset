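; Weapon object Blueprint with helper functions for choosing a compatible magazine for the weapon.
; IterateCompatibleMagazines filters a magazine array down to those whose MagType appears in the CompatibleMags list.
; FindBiggestMag keeps magazines holding more ammo than the given weapon's current ammo, then selects the fullest one.
; It returns that magazine with a validity flag indicating whether one was found.
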(fn IterateCompatibleMagazines
  (params (MagazineArray :type Array%20of%20Bp%20Magazine%20Object%20Object%20References) (Player :type BP%20True%20Fps%20Character%20Object%20Reference))
  (bind _array_element (Utilities|Array|ForEachLoopwithBreak MagazineArray)
    (:LoopBody
      (bind _array_element_2 (Utilities|Array|ForEachLoopwithBreak (Variables|WeaponInfo|GetCompatibleMags))
        (:LoopBody
          (if (Utilities|Enum|Equal(Enum) _array_element_2 (Variables|/Game/Blueprints/items/Magazines/Bp_Magazine_object.Bp_Magazine_object_C|GetMagType _array_element))
            (Utilities|Array|Add (LocalVariables|GetMagazineComparisonArray%28local%29) _array_element)))))
    (:Completed
      (return (LocalVariables|GetMagazineComparisonArray%28local%29)))))

(fn FindBiggestMag
  (params (MagazineArray :type Array%20of%20Bp%20Magazine%20Object%20Object%20References) (WeaponObjectRef :type Bp%20Weapon%20Object%20Object%20Reference))
  (bind _comparemagarray (LocalVariables|GetCompareMagArray))
  (if (Utilities|Array|IsNotEmpty MagazineArray)
    (Utilities|FlowControl|Sequence
      (:then_0
        (for _array_element MagazineArray
          (if (> (Variables|/Game/Blueprints/items/Magazines/Bp_Magazine_object.Bp_Magazine_object_C|GetCurrentAmmo _array_element) (Variables|Bp_Weapon_Object_C|GetCurrentAmmo WeaponObjectRef))
            (Utilities|Array|Add (LocalVariables|GetCompareMagArray) _array_element))))
      (:then_1
        (if (Utilities|Array|IsNotEmpty _comparemagarray)
          (bind (_array_element_2 _array_index) (Utilities|Array|ForEachLoopwithBreak _comparemagarray)
            (:LoopBody
              (if (> (Variables|/Game/Blueprints/items/Magazines/Bp_Magazine_object.Bp_Magazine_object_C|GetCurrentAmmo _array_element_2) (LocalVariables|GetMagCompareInteger%28local%29))
                (LocalVariables|SetMagCompareInteger%28local%29 (Variables|/Game/Blueprints/items/Magazines/Bp_Magazine_object.Bp_Magazine_object_C|GetCurrentAmmo _array_element_2))
                (LocalVariables|SetIndexOfMag%28local%29 _array_index)
                (LocalVariables|SetSelectedMagazine _array_element_2))))
          (else
            (return (LocalVariables|GetSelectedMagazine) (Utilities|IsValid (LocalVariables|GetSelectedMagazine))))))
      (:then_2
        (return (LocalVariables|GetSelectedMagazine) (Utilities|IsValid (LocalVariables|GetSelectedMagazine)))))
    (else
      (return (LocalVariables|GetSelectedMagazine) (Utilities|IsValid (LocalVariables|GetSelectedMagazine))))))