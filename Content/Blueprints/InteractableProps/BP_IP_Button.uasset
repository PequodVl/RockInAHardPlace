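; Interactable button prop that toggles the level's sun between a dim blue, night-like look and a bright white one.
; Each OnInteracted event runs a FlipFlop that swaps the visibility of two point lights and plays audio.
; Both branches find the DirectionalLight with display name "SunPosition", then set its color and intensity, applying the same rotation either way.
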(event EventBeginPlay
  (|CallParentFunction) ; This node is disabled and will not be called.\nDrag off pins to build functionality.
)

(event Collision|EventActorBeginOverlap
  (params (OtherActor :type Actor%20Object%20Reference)))

(event EventTick
  (params (DeltaSeconds :type Float%20%28single-precision%29)))

(event EventOnInteracted
  (params (Player :type BP%20True%20Fps%20Character%20Object%20Reference))
  (bind _pointlight (Variables|Default|GetPointLight))
  (bind _pointlight1 (Variables|Default|GetPointLight1))
  (Utilities|FlowControl|FlipFlop
    (:A
      (Rendering|SetVisibility _pointlight false false)
      (Rendering|SetVisibility _pointlight1 true false)
      (Audio|Components|Audio|Play (Variables|Default|GetAudio) 0.0)
      (bind _outactors (Actor|GetAllActorsOfClass "/Script/Engine.DirectionalLight"))
      (bind _array_element (Utilities|Array|ForEachLoopwithBreak _outactors :!label _label)
        (:LoopBody
          (if (Utilities|Enum|Equal(Enum) (Utilities|GetDisplayName _array_element) "SunPosition")
            (Transformation|SetActorRotation _array_element "-51.000000,-12.000000,21.000000")
            (Rendering|Components|Light|SetLightColor (Variables|/Script/Engine.Light|GetLightComponent _array_element) "(R=0.068359,G=0.284467,B=0.625000,A=1.000000)" true)
            (Rendering|Components|Light|SetIntensity (Variables|/Script/Engine.Light|GetLightComponent _array_element) 0.5)
            (goto _label Break)))))
    (:B
      (Rendering|SetVisibility _pointlight true false)
      (Rendering|SetVisibility _pointlight1 false false)
      (Audio|Components|Audio|Play (Variables|Default|GetAudio) 0.0)
      (bind _outactors_2 (Actor|GetAllActorsOfClass "/Script/Engine.DirectionalLight"))
      (bind _array_element_2 (Utilities|Array|ForEachLoopwithBreak _outactors_2 :!label _label_2)
        (:LoopBody
          (if (Utilities|Enum|Equal(Enum) (Utilities|GetDisplayName _array_element_2) "SunPosition")
            (Transformation|SetActorRotation _array_element_2 "-51.000000,-12.000000,21.000000")
            (Rendering|Components|Light|SetLightColor (Variables|/Script/Engine.Light|GetLightComponent _array_element_2) "(R=1.000000,G=1.000000,B=1.000000,A=1.000000)" true)
            (Rendering|Components|Light|SetIntensity (Variables|/Script/Engine.Light|GetLightComponent _array_element_2) 3e+01)
            (goto _label_2 Break)))))))

(fn ConstructionScript
  (|CallParentFunction))