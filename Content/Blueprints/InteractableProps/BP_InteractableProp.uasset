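; BP_InteractableProp is an interactable prop that shows an on-screen interaction widget while the player's cursor is on it.
; Cursor focus creates an IW_Interact widget with the item's name and image, placed in a screen-space component snapped to the attach point, defaulting to the root.
; Losing focus or leaving interaction range destroys that component.
; Interaction, range-entry and the text and default-item getters are empty stubs.
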(event EventBeginPlay)

(event EventOnItemIsinCursor
  (params (Player :type BP%20True%20Fps%20Character%20Object%20Reference))
  (Variables|Default|GetTheInteractionWidgetComponent
    (:then)
    (:else
      (bind _returnvalue (UserInterface|CreateWidget "/Game/Blueprints/Interface/IW_Interact.IW_Interact_C" (.AsPlayer%20Controller (Utilities|Casting|CastToPlayerController (Pawn|GetController Player))) (Variables|ItemInfo|GetItemName) (Variables|ItemInfo|GetItemImage)))
      (bind _returnvalue_2 (AddComponent|AddWidgetComponent false))
      (bind _output_get (Variables|Default|SetTheInteractionWidgetComponent _returnvalue_2))
      (UserInterface|SetWidget _output_get _returnvalue)
      (Class|WidgetComponent|SetWidgetSpace _output_get "Screen")
      (Class|WidgetComponent|SetDrawatDesiredSize _output_get true)
      (Collision|SetCollisionEnabled _output_get "NoCollision")
      (Transformation|AttachComponentToComponent _output_get (CallFunction|GetInteractionTextAttach) "None" "SnapToTarget" "SnapToTarget" "SnapToTarget" true))))

(event EventOnItemlostCursor
  (bind _theinteractionwidgetcomponent (Variables|Default|GetTheInteractionWidgetComponent)
    (:then
      (Components|DestroyComponent _theinteractionwidgetcomponent))
    (:else)))

(event EventOnInteractionRangeExited
  (bind _theinteractionwidgetcomponent (Variables|Default|GetTheInteractionWidgetComponent)
    (:then
      (Components|DestroyComponent _theinteractionwidgetcomponent))
    (:else)))

(event EventOnInteractionRangeEntered
  (params (Player :type BP%20True%20Fps%20Character%20Object%20Reference)))

(event EventOnInteracted
  (params (Player :type BP%20True%20Fps%20Character%20Object%20Reference)))

(fn ConstructionScript)

(fn GetInteractionText
  (return ""))

(fn GetInteractionTextAttach
  (return (Variables|Default|GetDefaultSceneRoot)))

(fn GetDefaultItemObject
  (return 0))